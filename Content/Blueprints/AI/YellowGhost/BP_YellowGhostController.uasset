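; AI controller for the yellow ghost in a Pac-Man game, which runs the BT_YellowGhost behavior tree on BeginPlay.
; Tick fetches the PacmanGameState and checks that its Grid is valid, then does nothing further.
; Disconnected leftover nodes look up the ghost's and Pac-Man's grid tiles and write a zero tiles-to-Pacman blackboard value with a debug print, none of which runs.
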(event `self.ReceiveBeginPlay`
  (`self.RunBehaviorTree` "/Game/Blueprints/AI/YellowGhost/Behaviour/BT_YellowGhost.BT_YellowGhost"))

(event `self.ReceiveTick`
  (params (DeltaSeconds :type "Float (single-precision)"))
  (bind _aspacman_game_state (cast `PacmanGameState` (`GameplayStatics.GetGameState`)))
  (if (`KismetSystemLibrary.IsValid` (`PacmanGameState.Grid` _aspacman_game_state))
    _))

(fn `UserConstructionScript`)